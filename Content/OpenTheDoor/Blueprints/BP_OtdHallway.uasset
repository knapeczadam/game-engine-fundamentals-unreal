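; BP_OtdHallway is a hallway actor that plays a room-completed sound and can display a running time counter.
; The sound plays when the player character overlaps its audio trigger.
; A one-second Delay on Tick throttles a counter that updates the time text roughly every second.
; The construction script assigns the configurable sound, initializes the text and hides it when time display is disabled.
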(event OnComponentBeginOverlap(AudioTrigger)
  (params (OverlappedComponent :type Primitive%20Component%20Object%20Reference) (OtherActor :type Actor%20Object%20Reference) (OtherComp :type Primitive%20Component%20Object%20Reference) (OtherBodyIndex :type Integer) (bFromSweep :type Boolean) (SweepResult :type Hit%20Result%20Structure%20%28by%20ref%29))
  (Utilities|IsValid OtherActor
    (:Is%20Valid
      (Utilities|Casting|CastToBP_OtdPlayerCharacter OtherActor)
      (Audio|Components|Audio|Play (Variables|Default|GetRoomCompletedSound) 0.0))))

(event EventTick
  (params (DeltaSeconds :type Float%20%28single-precision%29))
  (Utilities|FlowControl|Delay 1.0)
  (bind _result (Math|Integer|IncrementInt (Variables|Text|GetMeasuredTime))
    (:%20%20
      (bind _output_get (Variables|Text|SetMeasuredTime _result))
      (Rendering|Components|TextRender|SetText (Variables|Default|GetTimeText) (Utilities|Text|ToText(Integer) _output_get)))))

(fn ConstructionScript
  (bind _timetext (Variables|Default|GetTimeText))
  ;[0 0 0] Sound
  (Audio|Components|Audio|SetSound (Variables|Default|GetRoomCompletedSound) (Variables|Sound|GetSound))
  ;[0 0 0] Text
  (Rendering|Components|TextRender|SetText _timetext (Utilities|Text|ToText(Integer) (Variables|Text|GetMeasuredTime)))
  (if (not (Variables|Text|GetbShowMeasuredTime))
    (Rendering|SetVisibility _timetext false false)))