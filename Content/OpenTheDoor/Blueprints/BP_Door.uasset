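; BP_Door is a sliding double door with a rotating lock, opened and closed through the OpenDoor and CloseDoor events.
; A single Openclose timeline rotates the lock and slides both panels apart in mirrored directions, and CloseDoor reverses it.
; Opening switches the lock to a glass material; when the reverse finishes, the lock gets the UE logo material back and CallDoorCloseEvent is called.
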(event Custom|OpenDoor
  (Rendering|Material|SetMaterial (Variables|Default|GetLock) 0 "/Game/OpenTheDoor/Materials/MI_GlassDoor.MI_GlassDoor")
  (bind (_direction _lock_rotation _door_movement) (Timeline|Open/close Play)
    (:Update
      (Transformation|SetRelativeRotation (Variables|Default|GetLock) (Math|Rotator|MakeRotator _lock_rotation 0.0 0.0) false false)
      (Transformation|SetRelativeLocation (Variables|Default|GetRightDoor) (Math|Vector|MakeVector 0.0 _door_movement 0.0) false false)
      (Transformation|SetRelativeLocation (Variables|Default|GetLeftDoor) (Math|Vector|MakeVector 0.0 (* _door_movement -1.0) 0.0) false false))
    (:Finished
      (if (Utilities|Enum|Equal(Enum) _direction "Backward")
        (Rendering|Material|SetMaterial (Variables|Default|GetLock) 0 "/Game/OpenTheDoor/Materials/M_UELogoDoor.M_UELogoDoor")
        (Default|CallDoorCloseEvent)))))

(event Custom|CloseDoor
  (bind (_direction _lock_rotation _door_movement) (Timeline|Open/close Reverse)
    (:Update
      (Transformation|SetRelativeRotation (Variables|Default|GetLock) (Math|Rotator|MakeRotator _lock_rotation 0.0 0.0) false false)
      (Transformation|SetRelativeLocation (Variables|Default|GetRightDoor) (Math|Vector|MakeVector 0.0 _door_movement 0.0) false false)
      (Transformation|SetRelativeLocation (Variables|Default|GetLeftDoor) (Math|Vector|MakeVector 0.0 (* _door_movement -1.0) 0.0) false false))
    (:Finished
      (if (Utilities|Enum|Equal(Enum) _direction "Backward")
        (Rendering|Material|SetMaterial (Variables|Default|GetLock) 0 "/Game/OpenTheDoor/Materials/M_UELogoDoor.M_UELogoDoor")
        (Default|CallDoorCloseEvent)))))

(fn ConstructionScript)