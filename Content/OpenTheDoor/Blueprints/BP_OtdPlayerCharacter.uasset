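; BP_OtdPlayerCharacter is the player character for OpenTheDoor, with an early, debug-stage interaction system and respawn on destruction.
; Primary fire calls CheckTrace, a debug-drawn Visibility line trace from the camera out to InteractionDistance, and prints the hit actor's name if it has the "Pickup" tag.
; Secondary fire only prints a placeholder message.
; BeginPlay binds the destroyed event, which asks BP_OtdGameMode to respawn the player.
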(event Custom|OnDestroyed_Event
  (params (DestroyedActor :type Actor%20Object%20Reference))
  ;[0 0 0] Respawn player
  (bind _asbp_otd_game_mode (Utilities|Casting|CastToBP_OtdGameMode (Game|GetGameMode)))
  (Default|RespawnPlayer _asbp_otd_game_mode))

(event Input|EnhancedActionEvents|EnhancedInputActionIA_OtdFirePrimary
  (params (ActionValue :type Boolean) (ElapsedSeconds :type Float%20%28double-precision%29) (TriggeredSeconds :type Float%20%28double-precision%29) (InputAction :type Input%20Action%20Object%20Reference :default "/Game/OpenTheDoor/Input/Actions/IA_OtdFirePrimary.IA_OtdFirePrimary"))
  ;[0 0 0] Left mouse (primary mouse action)
  (:Started
    (bind (_hitobject _location _bpickup) (CallFunction|CheckTrace))
    (if _bpickup
      (Development|PrintString (Utilities|GetDisplayName _hitobject)))))

(event Input|EnhancedActionEvents|EnhancedInputActionIA_OtdFireSecondary
  (params (ActionValue :type Boolean) (ElapsedSeconds :type Float%20%28double-precision%29) (TriggeredSeconds :type Float%20%28double-precision%29) (InputAction :type Input%20Action%20Object%20Reference :default "/Game/OpenTheDoor/Input/Actions/IA_OtdFireSecondary.IA_OtdFireSecondary"))
  ;[0 0 0] Right mouse (secondary mouse action)
  (:Started
    (Development|PrintString "fire secondary")))

(event EventBeginPlay
  ;[0 0 0] Respawn player
  (EventDispatchers|BindEventtoOnDestroyed (delegate Custom|OnDestroyed_Event)))

(fn ConstructionScript
  (|CallParentFunction))

(fn CheckTrace
  (bind _returnvalue (Game|GetPlayerCameraManager 0))
  (bind _returnvalue_2 (Transformation|GetActorLocation _returnvalue))
  (bind (_outhit _returnvalue_3) (Collision|LineTraceByChannel _returnvalue_2 (+ _returnvalue_2 (* (Math|Vector|Normalize (Math|Rotator|GetRotationXVector (Transformation|GetActorRotation _returnvalue))) (Variables|Default|GetInteractionDistance))) "TraceTypeQuery1" false 0 "ForDuration"))
  (if _returnvalue_3
    (Utilities|IsValid (.HitActor (Collision|BreakHitResult _outhit))
      (:Is%20Valid
        (return (.HitActor (Collision|BreakHitResult _outhit)) (.Location (Collision|BreakHitResult _outhit)) (Actor|ActorHasTag (.HitActor (Collision|BreakHitResult _outhit)) "Pickup"))))
    (else
      (return 0 "0, 0, 0" false))))