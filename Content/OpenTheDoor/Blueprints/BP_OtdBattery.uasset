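; BP_OtdBattery is a battery actor in OpenTheDoor that carries a red, green or blue color state.
; Its construction script assigns the battery mesh and stores a dynamic instance of M_OtdBattery.
; SetColor clears the three color booleans, then sets the one matching the given index, without touching the material.
; The event graph has no active logic.
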(event EventBeginPlay)

(event Collision|EventActorBeginOverlap
  (params (OtherActor :type Actor%20Object%20Reference)))

(event EventTick
  (params (DeltaSeconds :type Float%20%28single-precision%29)))

(fn ConstructionScript
  (bind _battery (Variables|Default|GetBattery))
  (Components|StaticMesh|SetStaticMesh _battery (Variables|Default|GetBatteryMesh))
  (bind _returnvalue (Rendering|Material|CreateDynamicMaterialInstance _battery 0 "/Game/OpenTheDoor/Materials/M_OtdBattery.M_OtdBattery" "None" :!class /Script/Engine.PrimitiveComponent))
  (Variables|Default|SetBatteryMaterial _returnvalue))

(fn SetColor
  (params (ColorIndex :type Integer))
  (Utilities|FlowControl|Sequence
    (:then_0
      (Variables|Default|SetbRed false))
    (:then_1
      (Variables|Default|SetbGreen false))
    (:then_2
      (Variables|Default|SetbBlue false))
    (:then_3
      (switch int ColorIndex
        (:0
          (Variables|Default|SetbRed true))
        (:1
          (Variables|Default|SetbGreen true))
        (:2
          (Variables|Default|SetbBlue true))))))