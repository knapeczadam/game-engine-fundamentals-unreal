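; BP_OtdButton is a color-cycling button that recolors a battery docked on it in OpenTheDoor.
; A tagged battery entering Box1 makes the player drop it, then it stops simulating physics and snaps above the box until it leaves.
; Each press applies the current color and index to the docked battery, then advances the wrapping index.
; A dynamic material instance displays the color the next press will apply.
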(event OnComponentBeginOverlap(Box1)
  (params (OverlappedComponent :type Primitive%20Component%20Object%20Reference) (OtherActor :type Actor%20Object%20Reference) (OtherComp :type Primitive%20Component%20Object%20Reference) (OtherBodyIndex :type Integer) (bFromSweep :type Boolean) (SweepResult :type Hit%20Result%20Structure%20%28by%20ref%29))
  (if (Actor|ActorHasTag OtherActor "battery")
    (bind _asbp_otd_player_character (Utilities|Casting|CastToBP_OtdPlayerCharacter (Game|Player|GetPlayerPawn 0)))
    (Default|DropObject _asbp_otd_player_character)
    (bind _asbp_otd_battery (Utilities|Casting|CastToBP_OtdBattery OtherActor))
    (Variables|Default|SetBattery _asbp_otd_battery)
    (Physics|SetSimulatePhysics (Variables|/Game/OpenTheDoor/Blueprints/BP_OtdBattery.BP_OtdBattery_C|GetBattery _asbp_otd_battery) false)
    (Transformation|SetWorldLocationAndRotation (Variables|/Game/OpenTheDoor/Blueprints/BP_OtdBattery.BP_OtdBattery_C|GetBattery _asbp_otd_battery) (+ (Transformation|GetWorldLocation (Variables|Default|GetBox1)) (Math|Vector|MakeVector 0.0 0.0 5e+01)) "0, 0, 0" false false)
    (Variables|Default|SetbBatteryAttached true)))

(event OnComponentEndOverlap(Box1)
  (params (OverlappedComponent :type Primitive%20Component%20Object%20Reference) (OtherActor :type Actor%20Object%20Reference) (OtherComp :type Primitive%20Component%20Object%20Reference) (OtherBodyIndex :type Integer))
  (if (Actor|ActorHasTag OtherActor "battery")
    (Variables|Default|SetbBatteryAttached false)
    (Variables|Default|SetBattery 0)))

(event Custom|OnButtonPress
  (bind _battery (Variables|Default|GetBattery))
  (Utilities|FlowControl|Sequence
    (:then_0
      (if (Variables|Default|GetbBatteryAttached)
        (Utilities|IsValid _battery
          (:Is%20Valid
            (Rendering|Material|SetVectorParameterValue (Variables|/Game/OpenTheDoor/Blueprints/BP_OtdBattery.BP_OtdBattery_C|GetBatteryMaterial _battery) "Color2" (Utilities|Array|Get(acopy) (Variables|Default|GetButtonColors) (Variables|Default|GetColorIndex)) :!class /Script/Engine.MaterialInstanceDynamic)
            (Default|SetColor (Variables|Default|GetBattery) (Variables|Default|GetColorIndex))))))
    (:then_1
      (bind _result (Math|Integer|IncrementInt (Variables|Default|GetColorIndex))
        (:%20%20
          (bind _output_get (Variables|Default|SetColorIndex _result))
          (if (> _output_get (Utilities|Array|LastIndex (Variables|Default|GetButtonColors)))
            (Variables|Default|SetColorIndex 0))
          (Rendering|Material|SetVectorParameterValue (Variables|Default|GetButtonMaterial) "ColorActive" (Utilities|Array|Get(acopy) (Variables|Default|GetButtonColors) (Variables|Default|GetColorIndex)) :!class /Script/Engine.MaterialInstanceDynamic))))))

(fn ConstructionScript
  (bind _returnvalue (Rendering|Material|CreateDynamicMaterialInstance (Variables|Default|GetButton) 1 "/Game/OpenTheDoor/Materials/M_OtdButton.M_OtdButton" "None" :!class /Script/Engine.PrimitiveComponent))
  (bind _output_get (Variables|Default|SetButtonMaterial _returnvalue))
  (Rendering|Material|SetVectorParameterValue _output_get "ColorActive" (Utilities|Array|Get(acopy) (Variables|Default|GetButtonColors)) :!class /Script/Engine.MaterialInstanceDynamic))