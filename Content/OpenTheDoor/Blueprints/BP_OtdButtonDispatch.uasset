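; Pressure button for OpenTheDoor that broadcasts a ButtonPressed event dispatcher.
; Overlapping the Trigger plays the Press timeline and ending the overlap reverses it.
; The timeline moves ButtonBase along Z and blends the emissive color of a dynamic material, created in the construction script, from black to orange.
; The dispatcher fires only when the timeline finishes in the forward direction, so a completed release stays silent.
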(event OnComponentBeginOverlap(Trigger)
  (params (OverlappedComponent :type Primitive%20Component%20Object%20Reference) (OtherActor :type Actor%20Object%20Reference) (OtherComp :type Primitive%20Component%20Object%20Reference) (OtherBodyIndex :type Integer) (bFromSweep :type Boolean) (SweepResult :type Hit%20Result%20Structure%20%28by%20ref%29))
  (bind (_direction _press _glow) (Timeline|Press Play)
    (:Update
      (Transformation|SetRelativeLocation (Variables|Default|GetButtonBase) (Math|Vector|MakeVector 0.0 0.0 (/ _press 1.5)) false false)
      (Rendering|Material|SetVectorParameterValue (Variables|Default|GetButtonMaterial) "Emissive Color" (Math|Color|Lerp(LinearColor) :B "(R=0.600000,G=0.329412,B=0.000000,A=1.000000)" :Alpha _glow) :!class /Script/Engine.MaterialInstanceDynamic))
    (:Finished
      (switch Utilities|FlowControl|Switch|SwitchonETimelineDirection _direction
        (:Forward
          (Default|CallButtonPressed))))))

(event OnComponentEndOverlap(Trigger)
  (params (OverlappedComponent :type Primitive%20Component%20Object%20Reference) (OtherActor :type Actor%20Object%20Reference) (OtherComp :type Primitive%20Component%20Object%20Reference) (OtherBodyIndex :type Integer))
  (bind (_direction _press _glow) (Timeline|Press Reverse)
    (:Update
      (Transformation|SetRelativeLocation (Variables|Default|GetButtonBase) (Math|Vector|MakeVector 0.0 0.0 (/ _press 1.5)) false false)
      (Rendering|Material|SetVectorParameterValue (Variables|Default|GetButtonMaterial) "Emissive Color" (Math|Color|Lerp(LinearColor) :B "(R=0.600000,G=0.329412,B=0.000000,A=1.000000)" :Alpha _glow) :!class /Script/Engine.MaterialInstanceDynamic))
    (:Finished
      (switch Utilities|FlowControl|Switch|SwitchonETimelineDirection _direction
        (:Forward
          (Default|CallButtonPressed))))))

(fn ConstructionScript
  (bind _returnvalue (Rendering|Material|CreateDynamicMaterialInstance (Variables|Default|GetButtonBase) 0 0 "None" :!class /Script/Engine.PrimitiveComponent))
  (Variables|Default|SetButtonMaterial _returnvalue))