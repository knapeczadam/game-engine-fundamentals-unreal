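; BP_OtdWall is a wall Blueprint for the OpenTheDoor game that can start hidden and appear later.
; On BeginPlay, if HideWallOnStart is set, it hides the Wall component and turns off its collision and component tick.
; The EnableWall event reverses this, making the wall visible, restoring query-and-physics collision and re-enabling its tick.
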(event Custom|EnableWall
  (bind _wall (Variables|Default|GetWall))
  (Rendering|SetVisibility _wall true false)
  (Collision|SetCollisionEnabled _wall "QueryAndPhysics")
  (Components|Tick|SetComponentTickEnabled _wall true))

(event EventBeginPlay
  (bind _wall (Variables|Default|GetWall))
  (if (Variables|Default|GetbHideWallOnStart)
    (Rendering|SetVisibility _wall false false)
    (Collision|SetCollisionEnabled _wall "NoCollision")
    (Components|Tick|SetComponentTickEnabled _wall false)))

(fn ConstructionScript)