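; Color-mixing puzzle door that lets AI pass only when its color matches CorrectColor.
; Left and right trigger volumes each take one battery from the player, snap it in place with physics off, and read its color.
; UpdateColor mixes both colors additively (white when empty), tints a dynamic material, and fires correct/incorrect dispatchers.
; The door binds these dispatchers to toggle AiCollision between Overlap and Block on a custom collision channel.
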(event OnComponentBeginOverlap(CollisionRight)
  (params (OverlappedComponent :type Primitive%20Component%20Object%20Reference) (OtherActor :type Actor%20Object%20Reference) (OtherComp :type Primitive%20Component%20Object%20Reference) (OtherBodyIndex :type Integer) (bFromSweep :type Boolean) (SweepResult :type Hit%20Result%20Structure%20%28by%20ref%29))
  (if (Actor|ActorHasTag OtherActor "battery")
    (Utilities|IsValid (Variables|Default|GetBatteryRight)
      (:Is%20Not%20Valid
        (bind _asbp_otd_battery (Utilities|Casting|CastToBP_OtdBattery OtherActor))
        (Variables|Default|SetBatteryRight _asbp_otd_battery)
        (bind _asbp_otd_player_character (Utilities|Casting|CastToBP_OtdPlayerCharacter (Game|Player|GetPlayerPawn 0)))
        (Default|DropObject _asbp_otd_player_character)
        (Physics|SetSimulatePhysics (Variables|/Game/OpenTheDoor/Blueprints/BP_OtdBattery.BP_OtdBattery_C|GetBattery (Variables|Default|GetBatteryRight)) false)
        (Transformation|SetWorldLocationAndRotation (Variables|/Game/OpenTheDoor/Blueprints/BP_OtdBattery.BP_OtdBattery_C|GetBattery (Variables|Default|GetBatteryRight)) (+ (Transformation|GetWorldLocation (Variables|Default|GetCollisionRight)) "0.000000,0.000000,30.000000") "0, 0, 0" false false)
        (bind _color (Default|GetColor (Variables|Default|GetBatteryRight)))
        (Variables|Default|SetColor2 _color)
        (CallFunction|UpdateColor)))))

(event OnComponentEndOverlap(CollisionRight)
  (params (OverlappedComponent :type Primitive%20Component%20Object%20Reference) (OtherActor :type Actor%20Object%20Reference) (OtherComp :type Primitive%20Component%20Object%20Reference) (OtherBodyIndex :type Integer))
  (if (Actor|ActorHasTag OtherActor "battery")
    (bind _asbp_otd_battery (Utilities|Casting|CastToBP_OtdBattery OtherActor))
    (if (== _asbp_otd_battery (Variables|Default|GetBatteryRight))
      (Variables|Default|SetBatteryRight 0)
      (Variables|Default|SetColor2 "NewEnumerator3")
      (CallFunction|UpdateColor))))

(event OnComponentBeginOverlap(CollisionLeft)
  (params (OverlappedComponent :type Primitive%20Component%20Object%20Reference) (OtherActor :type Actor%20Object%20Reference) (OtherComp :type Primitive%20Component%20Object%20Reference) (OtherBodyIndex :type Integer) (bFromSweep :type Boolean) (SweepResult :type Hit%20Result%20Structure%20%28by%20ref%29))
  (if (Actor|ActorHasTag OtherActor "battery")
    (Utilities|IsValid (Variables|Default|GetBatteryLeft)
      (:Is%20Not%20Valid
        (bind _asbp_otd_battery (Utilities|Casting|CastToBP_OtdBattery OtherActor))
        (Variables|Default|SetBatteryLeft _asbp_otd_battery)
        (bind _asbp_otd_player_character (Utilities|Casting|CastToBP_OtdPlayerCharacter (Game|Player|GetPlayerPawn 0)))
        (Default|DropObject _asbp_otd_player_character)
        (Physics|SetSimulatePhysics (Variables|/Game/OpenTheDoor/Blueprints/BP_OtdBattery.BP_OtdBattery_C|GetBattery (Variables|Default|GetBatteryLeft)) false)
        (Transformation|SetWorldLocationAndRotation (Variables|/Game/OpenTheDoor/Blueprints/BP_OtdBattery.BP_OtdBattery_C|GetBattery (Variables|Default|GetBatteryLeft)) (+ (Transformation|GetWorldLocation (Variables|Default|GetCollisionLeft)) "0.000000,0.000000,30.000000") "0, 0, 0" false false)
        (bind _color (Default|GetColor (Variables|Default|GetBatteryLeft)))
        (Variables|Default|SetColor1 _color)
        (CallFunction|UpdateColor)))))

(event OnComponentEndOverlap(CollisionLeft)
  (params (OverlappedComponent :type Primitive%20Component%20Object%20Reference) (OtherActor :type Actor%20Object%20Reference) (OtherComp :type Primitive%20Component%20Object%20Reference) (OtherBodyIndex :type Integer))
  (if (Actor|ActorHasTag OtherActor "battery")
    (bind _asbp_otd_battery (Utilities|Casting|CastToBP_OtdBattery OtherActor))
    (if (== _asbp_otd_battery (Variables|Default|GetBatteryLeft))
      (Variables|Default|SetBatteryLeft 0)
      (Variables|Default|SetColor1 "NewEnumerator3")
      (CallFunction|UpdateColor))))

(event Custom|BlockAi
  (Collision|SetCollisionResponsetoChannel (Variables|Default|GetAiCollision) "ECC_GameTraceChannel2" "ECR_Block"))

(event Custom|AllowAiToPass
  (Collision|SetCollisionResponsetoChannel (Variables|Default|GetAiCollision) "ECC_GameTraceChannel2" "ECR_Overlap"))

(event EventBeginPlay
  (EventDispatchers|BindEventtoOnCorrectColor (delegate Custom|AllowAiToPass))
  (EventDispatchers|BindEventtoOnIncorrectColor (delegate Custom|BlockAi))
  (CallFunction|UpdateColor))

(fn ConstructionScript
  (bind _returnvalue (Rendering|Material|CreateDynamicMaterialInstance (Variables|Default|GetDoor) 0 0 "None" :!class /Script/Engine.PrimitiveComponent))
  (Variables|Default|SetDoorColor _returnvalue))

(fn SetColor1
  (params (Color :type EColor%20Enum :default "NewEnumerator0"))
  (Variables|Default|SetColor1 Color)
  (CallFunction|UpdateColor))

(fn SetColor2
  (params (Color :type EColor%20Enum :default "NewEnumerator0"))
  (Variables|Default|SetColor2 Color)
  (CallFunction|UpdateColor))

(fn UpdateColor
  (bind _doorcolor (Variables|Default|GetDoorColor))
  (if (or (Utilities|Enum|Equal(Enum) (Variables|Default|GetColor1) "NewEnumerator3") (Utilities|Enum|Equal(Enum) (Variables|Default|GetColor2) "NewEnumerator3"))
    (if (and (Utilities|Enum|Equal(Enum) (Variables|Default|GetColor1) "NewEnumerator3") (Utilities|Enum|Equal(Enum) (Variables|Default|GetColor2) "NewEnumerator3"))
      (Rendering|Material|SetVectorParameterValue _doorcolor "Color" "(R=1.000000,G=1.000000,B=1.000000,A=1.000000)" :!class /Script/Engine.MaterialInstanceDynamic)
      (if (Utilities|Enum|Equal(Enum) (Variables|Default|GetCorrectColor) "NewEnumerator3")
        (Default|CallOnCorrectColor)
        (else
          (Default|CallOnIncorrectColor)))
      (elif (Utilities|Enum|NotEqual(Enum) (Variables|Default|GetColor1) "NewEnumerator3")
        (switch Utilities|FlowControl|Switch|SwitchonEColor (Variables|Default|GetColor1)
          (:NewEnumerator0
            (Rendering|Material|SetVectorParameterValue _doorcolor "Color" "(R=1.000000,G=0.000000,B=0.000000,A=1.000000)" :!class /Script/Engine.MaterialInstanceDynamic :!label _label)
            (if (Utilities|Enum|Equal(Enum) (Variables|Default|GetCorrectColor) "NewEnumerator0")
              (Default|CallOnCorrectColor)
              (else
                (Default|CallOnIncorrectColor))))
          (:NewEnumerator1
            (Rendering|Material|SetVectorParameterValue _doorcolor "Color" "(R=0.000000,G=1.000000,B=0.000000,A=1.000000)" :!class /Script/Engine.MaterialInstanceDynamic :!label _label_2)
            (if (Utilities|Enum|Equal(Enum) (Variables|Default|GetCorrectColor) "NewEnumerator1")
              (Default|CallOnCorrectColor)
              (else
                (Default|CallOnIncorrectColor))))
          (:NewEnumerator2
            (Rendering|Material|SetVectorParameterValue _doorcolor "Color" "(R=0.000000,G=0.000000,B=1.000000,A=1.000000)" :!class /Script/Engine.MaterialInstanceDynamic :!label _label_3)
            (if (Utilities|Enum|Equal(Enum) (Variables|Default|GetCorrectColor) "NewEnumerator2")
              (Default|CallOnCorrectColor)
              (else
                (Default|CallOnIncorrectColor)))))
        (else
          (switch Utilities|FlowControl|Switch|SwitchonEColor (Variables|Default|GetColor2) :!label _label_4
            (:NewEnumerator0
              (goto _label))
            (:NewEnumerator1
              (goto _label_2))
            (:NewEnumerator2
              (goto _label_3))))))
    (elif (Utilities|Enum|Equal(Enum) (Variables|Default|GetColor1) (Variables|Default|GetColor2))
      (goto _label_4)
      (else
        ;[0 0 0] Yellow
        (if (or (and (Utilities|Enum|Equal(Enum) (Variables|Default|GetColor1) "NewEnumerator0") (Utilities|Enum|Equal(Enum) (Variables|Default|GetColor2) "NewEnumerator1")) (and (Utilities|Enum|Equal(Enum) (Variables|Default|GetColor1) "NewEnumerator1") (Utilities|Enum|Equal(Enum) (Variables|Default|GetColor2) "NewEnumerator0")))
          (Rendering|Material|SetVectorParameterValue (Variables|Default|GetDoorColor) "Color" "(R=1.000000,G=1.000000,B=0.000000,A=1.000000)" :!class /Script/Engine.MaterialInstanceDynamic)
          (if (Utilities|Enum|Equal(Enum) (Variables|Default|GetCorrectColor) "NewEnumerator4")
            (Default|CallOnCorrectColor)
            (else
              (Default|CallOnIncorrectColor)))
          (else
            ;[0 0 0] Magenta
            (if (or (and (Utilities|Enum|Equal(Enum) (Variables|Default|GetColor1) "NewEnumerator0") (Utilities|Enum|Equal(Enum) (Variables|Default|GetColor2) "NewEnumerator2")) (and (Utilities|Enum|Equal(Enum) (Variables|Default|GetColor1) "NewEnumerator2") (Utilities|Enum|Equal(Enum) (Variables|Default|GetColor2) "NewEnumerator0")))
              (Rendering|Material|SetVectorParameterValue (Variables|Default|GetDoorColor) "Color" "(R=1.000000,G=0.000000,B=1.000000,A=1.000000)" :!class /Script/Engine.MaterialInstanceDynamic)
              (if (Utilities|Enum|Equal(Enum) (Variables|Default|GetCorrectColor) "NewEnumerator6")
                (Default|CallOnCorrectColor)
                (else
                  (Default|CallOnIncorrectColor)))
              (else
                ;[0 0 0] Cyan
                (if (or (and (Utilities|Enum|Equal(Enum) (Variables|Default|GetColor1) "NewEnumerator1") (Utilities|Enum|Equal(Enum) (Variables|Default|GetColor2) "NewEnumerator2")) (and (Utilities|Enum|Equal(Enum) (Variables|Default|GetColor1) "NewEnumerator2") (Utilities|Enum|Equal(Enum) (Variables|Default|GetColor2) "NewEnumerator1")))
                  (Rendering|Material|SetVectorParameterValue (Variables|Default|GetDoorColor) "Color" "(R=0.000000,G=1.000000,B=1.000000,A=1.000000)" :!class /Script/Engine.MaterialInstanceDynamic)
                  (if (Utilities|Enum|Equal(Enum) (Variables|Default|GetCorrectColor) "NewEnumerator5")
                    (Default|CallOnCorrectColor)
                    (else
                      (Default|CallOnIncorrectColor))))))))))))